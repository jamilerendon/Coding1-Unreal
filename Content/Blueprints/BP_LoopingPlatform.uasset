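; BP_LoopingPlatform is a moving platform actor that travels between its Start and End points.
; On BeginPlay a Timeline starts playing, and its float track drives a transform lerp that sets the Platform's world location and rotation each update.
; The Timeline's Moving and Stopped events swap the platform material between active and ready looks.
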(event EventBeginPlay
  (bind _newtrack_0 (Timeline|Timeline Play)
    (:Update
      (Transformation|SetWorldLocationAndRotation (Variables|Default|GetPlatform) (.location (Math|Transform|Lerp(Transform) (Transformation|GetWorldTransform (Variables|Default|GetStart)) (Transformation|GetWorldTransform (Variables|Default|GetEnd)) _newtrack_0)) (.rotation (Math|Transform|Lerp(Transform) (Transformation|GetWorldTransform (Variables|Default|GetStart)) (Transformation|GetWorldTransform (Variables|Default|GetEnd)) _newtrack_0)) false false))
    (:Moving
      (Rendering|Material|SetMaterial (Variables|Default|GetPlatform) 0 "/Game/Materials/FallingPlatforms/M_ActivePlatform.M_ActivePlatform"))
    (:Stopped
      (Rendering|Material|SetMaterial (Variables|Default|GetPlatform) 0 "/Game/Materials/FallingPlatforms/M_ReadyPlatform.M_ReadyPlatform"))))

(event Collision|EventActorBeginOverlap
  (params (OtherActor :type Actor%20Object%20Reference)))

(event EventTick
  (params (DeltaSeconds :type Float%20%28single-precision%29)))

(fn ConstructionScript)